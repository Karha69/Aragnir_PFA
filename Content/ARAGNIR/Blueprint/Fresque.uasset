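; Fresque is a mural Blueprint that drives a dissolve effect on its static mesh based on the player's distance.
; Each Tick it measures from its Scene component to the ThirdPersonCharacter's capsule, scales and clamps that distance to 0–1, and feeds it into the "Fresque Dissolve" material parameter.
; It calls CreateDynamicMaterialInstance from Fresque_1 every frame rather than caching it, and prints a leftover constant debug string.
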(event `self.ReceiveTick`
  (params (DeltaSeconds :type "Float (single-precision)"))
  (bind _asthird_person_character (cast `/Game/ARAGNIR/Blueprint/ThirdPersonCharacter` (`GameplayStatics.GetPlayerCharacter` 0)))
  (bind _output_get (set `self.DistanceBetween` (- (`SceneComponent.K2_GetComponentLocation` (`self.Scene`)) (`SceneComponent.K2_GetComponentLocation` (`Character.CapsuleComponent` _asthird_person_character)))))
  (bind _returnvalue (`PrimitiveComponent.CreateDynamicMaterialInstance` (`self.StaticMeshComponent`) 0 "/Game/ARAGNIR/Marie/Environement/maps/fresque_1/fresque_1.fresque_1" "None"))
  (`MaterialInstanceDynamic.SetScalarParameterValue` _returnvalue "Fresque Dissolve" (`KismetMathLibrary.FClamp` (/ (`KismetMathLibrary.VSize` _output_get) 10000.0)))
  (`KismetSystemLibrary.PrintString` (`KismetStringLibrary.Conv_DoubleToString` 0.0)))

(fn `UserConstructionScript`)